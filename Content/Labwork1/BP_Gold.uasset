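; BP_Gold is a gold pickup that adds a random amount to PlayerGold in BP_GameMode when interacted with, then prints the total and destroys itself.
; The construction script rolls the amount, and the CreateMesh macro adds one to three static meshes by value threshold, each with randomized offset and scale.
; At BeginPlay it caches the game mode and positions a text label showing the amount.
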(event `self.ReceiveBeginPlay`
  (bind _textrender (`self.TextRender`))
  (bind _asbp_game_mode (cast `/Game/Labwork1/BP_GameMode` (`GameplayStatics.GetGameMode`)))
  (set `self.As BP Game Mode` _asbp_game_mode)
  (`TextRenderComponent.K2_SetText` (`self.TextRender`) (`KismetTextLibrary.Conv_IntToText` (`self.ItemGold`)))
  (`SceneComponent.K2_SetRelativeLocation` _textrender (25.0 -25.0 0.0) false false)
  (`SceneComponent.K2_SetRelativeLocation` (`self.TextRender`) (25.0 -25.0 0.0) false false)
  (`SceneComponent.K2_SetRelativeRotation` _textrender (struct :`Yaw` -90.0) false false))

(event `/Game/Labwork1/BPI_Interactable.Interact `
  (bind _output_get (set `/Game/Labwork1/BP_GameMode.PlayerGold` (+ (`/Game/Labwork1/BP_GameMode.PlayerGold` (`self.As BP Game Mode`)) (`self.ItemGold`)) (`self.As BP Game Mode`)))
  (`KismetSystemLibrary.PrintString` (`KismetStringLibrary.Concat_StrStr` "Current Gold" (`KismetStringLibrary.Conv_IntToString` _output_get)))
  (`self.K2_DestroyActor`))

(fn `UserConstructionScript`
  (bind _itemgold (`self.ItemGold`))
  (bind _output_get (set `self.ItemGold` (`KismetMathLibrary.RandomIntegerInRange` 1 99)))
  (`KismetSystemLibrary.PrintString` (`KismetStringLibrary.Conv_IntToString` _output_get))
  (`self.CreateMesh ` (>= _itemgold 76)
    (:`Out`
      _)
    (:`False`
      _))
  (`self.CreateMesh ` (>= _itemgold 26)
    (:`Out`
      _)
    (:`False`
      _))
  (`self.CreateMesh ` (>= _itemgold 1)))