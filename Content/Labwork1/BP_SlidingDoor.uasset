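; BP_SlidingDoor is an interactable door that slides open only when the game mode's Keys value equals its KeyNumber.
; BeginPlay caches BP_GameMode; a matching Interact plays the Door_Rotate timeline, which lerps the door mesh's relative location from StartLoc to FinishLoc.
; A mismatch prints a wrong-key message.
; The construction script picks the door material from KeyNumber, visually distinguishing the key types.
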(event `self.ReceiveBeginPlay`
  (bind _asbp_game_mode (cast `/Game/Labwork1/BP_GameMode` (`GameplayStatics.GetGameMode`)))
  (set `self.As BP Game Mode` _asbp_game_mode))

(event `/Game/Labwork1/BPI_Interactable.Interact `
  (if (== (`/Game/Labwork1/BP_GameMode.Keys` (`self.As BP Game Mode`)) (`self.KeyNumber`))
    (bind (_direction _newtrack_0) (`Timeline|Door_Rotate`)
      (:`Update`
        (`SceneComponent.K2_SetRelativeLocation` (`self.SM_Door`) (`KismetMathLibrary.VLerp` (`self.StartLoc`) (`self.FinishLoc`) _newtrack_0) false false)))
    (else
      (`KismetSystemLibrary.PrintString` "You don't have the correct key "))))

(fn `UserConstructionScript`
  (bind _sm_door (`self.SM_Door`))
  (switch `int` (`self.KeyNumber`)
    (:`0`
      (`PrimitiveComponent.SetMaterial` _sm_door 0 "/Game/StarterContent/Materials/M_Ground_Moss.M_Ground_Moss"))
    (:`1`
      (`PrimitiveComponent.SetMaterial` _sm_door 0 "/Game/StarterContent/Materials/M_Wood_Walnut.M_Wood_Walnut"))))