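; Spike trap actor that springs when the player enters its activation box and takes health from them on contact with its damage box.
; A timeline animates the spike mesh's height, while damage goes through the player character's HealthUpdate.
; It binds to the player's trap dispatcher on BeginPlay; a matching trap type permanently disarms it by lowering the spikes, disabling both boxes and destroying the timeline.
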(event `self.ReceiveBeginPlay`
  (bind _asbp_third_person_character (cast `/Game/ThirdPerson/Blueprints/BP_ThirdPersonCharacter` (`GameplayStatics.GetPlayerCharacter` 0)))
  (bind _output_get (set `self.As BP Third Person Character` _asbp_third_person_character))
  (add `/Game/ThirdPerson/Blueprints/BP_ThirdPersonCharacter.DP_Trap` _output_get (delegate `DP_Trap_Event`)))

(event `DP_Trap_Event`
  (params (TrapType :type "/Game/Labwork1/TrapType Enum" :default "NewEnumerator0"))
  (if (`|EnumEquality` TrapType (`self.Trap Type`))
    (`SceneComponent.K2_SetRelativeLocation` (`self.SpikeTrap_F4C46E73`) (0.0 0.0 -130.0) false false)
    (`PrimitiveComponent.SetCollisionEnabled` (`self.DamageBox`) "NoCollision")
    (`PrimitiveComponent.SetCollisionEnabled` (`self.ActivationBox`) "NoCollision")
    (`ActorComponent.K2_DestroyComponent` (`self.SpikesTL`))))

(event `self.DamageBox.OnComponentBeginOverlap`
  (params (OverlappedComponent :type "PrimitiveComponent Object Reference") (OtherActor :type "Actor Object Reference") (OtherComp :type "PrimitiveComponent Object Reference") (OtherBodyIndex :type Integer) (bFromSweep :type Boolean) (SweepResult :type "HitResult Structure (by ref)"))
  (bind _as_bp_third_person_character (`self.As BP Third Person Character`))
  (if (== OtherActor _as_bp_third_person_character)
    (`/Game/ThirdPerson/Blueprints/BP_ThirdPersonCharacter.HealthUpdate ` _as_bp_third_person_character -15.0)))

(event `self.ActivationBox.OnComponentBeginOverlap`
  (params (OverlappedComponent :type "PrimitiveComponent Object Reference") (OtherActor :type "Actor Object Reference") (OtherComp :type "PrimitiveComponent Object Reference") (OtherBodyIndex :type Integer) (bFromSweep :type Boolean) (SweepResult :type "HitResult Structure (by ref)"))
  (if (== OtherActor (`self.As BP Third Person Character`))
    (`self.SpikesTL`
      (:`then`
        (bind (_direction _newtrack_0) (`Timeline|SpikesTL`)
          (:`Update`
            (`SceneComponent.K2_SetRelativeLocation` (`self.SpikeTrap_F4C46E73`) (`KismetMathLibrary.MakeVector` 0.0 0.0 _newtrack_0) false false))))
      (:`else`))))

(fn `UserConstructionScript`)