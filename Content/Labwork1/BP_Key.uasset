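; BP_Key is an interactable key pickup that is identified by its KeyNumber.
; The construction script picks the sphere's material from KeyNumber, using moss for 0 and walnut for 1.
; On Interact it overwrites Keys on the cached BP_GameMode with its number, prints an acquired message with the matching name, then destroys itself.
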(event `self.ReceiveBeginPlay`
  (bind _asbp_game_mode (cast `/Game/Labwork1/BP_GameMode` (`GameplayStatics.GetGameMode`)))
  (set `self.As BP Game Mode` _asbp_game_mode))

(event `/Game/Labwork1/BPI_Interactable.Interact `
  (bind _output_get (set `/Game/Labwork1/BP_GameMode.Keys` (`self.KeyNumber`) (`self.As BP Game Mode`)))
  (`KismetSystemLibrary.PrintString` (`KismetStringLibrary.Concat_StrStr` "Key" (`|GetArrayItem` (`self.Names`) _output_get) "Acquired"))
  (`self.K2_DestroyActor`))

(fn `UserConstructionScript`
  (bind _sphere (`self.Sphere`))
  (switch `int` (`self.KeyNumber`)
    (:`0`
      (`PrimitiveComponent.SetMaterial` _sphere 0 "/Game/StarterContent/Materials/M_Ground_Moss.M_Ground_Moss"))
    (:`1`
      (`PrimitiveComponent.SetMaterial` _sphere 0 "/Game/StarterContent/Materials/M_Wood_Walnut.M_Wood_Walnut"))))